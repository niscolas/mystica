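; Gameplay ability that spawns a configurable weapon actor for its avatar and registers it with that avatar's combat setup.
; On activation it spawns the weapon class with the avatar as owner and instigator, then registers its weapon component by gameplay tag, optionally equipping it.
; It attaches the actor to the owning component at a configured socket, then ends.
; EndAbility is only reached when the spawn succeeds.
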(event `self.K2_ActivateAbility`
  (bind _returnvalue (`self.GetAvatarActorFromActorInfo`))
  (bind _returnvalue_2 (`|SpawnActorFromClass` (`self.WeaponClass`) (`KismetMathLibrary.MakeTransform` (0.0 0.0 0.0)) "AdjustIfPossibleButAlwaysSpawn" "MultiplyWithRoot" _returnvalue (cast `Pawn` _returnvalue :!pure true)))
  (`/Engine/EditorBlueprintResources/StandardMacros.IsValid` _returnvalue_2
    (:`Is Valid`
      (`CombatComponent.RegisterWeapon` (`self.GetCombatComponentFromActorInfo`) (`self.WeaponGameplayTag`) (`MysticaMiscFunctionLibrary.GetWeaponComponentFromActor` _returnvalue_2) (`self.ShouldEquipWeapon`))
      (`Actor.K2_AttachToComponent` _returnvalue_2 (`self.GetOwningComponentFromActorInfo`) (`self.AttachSocketName`) "SnapToTarget" "KeepRelative" "KeepWorld" true)
      (`self.K2_EndAbility`))))