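; Base Blueprint for orc enemies that handles the death sequence with a material dissolve before removing the actor.
; On Died it freezes animation and disables capsule collision, then waits for a configurable pre-dissolve delay.
; It then swaps the mesh's first material slot to a dissolve material, drives its Dissolve scalar parameter from a timeline, and destroys the actor when the timeline finishes.
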(event `/Game/_Main/Enemies/BPI_Enemy.Died`
  (set `SkeletalMeshComponent.bPauseAnims` true (`self.Mesh`))
  (`PrimitiveComponent.SetCollisionEnabled` (`self.CapsuleComponent`) "NoCollision")
  (`KismetSystemLibrary.Delay` (`self.PreDissolveDelay`))
  (`PrimitiveComponent.SetMaterial` (`self.Mesh`) 0 "/Game/_Main/Libraries/MaterialLibrary/MI_Dissolve_Default.MI_Dissolve_Default")
  (bind (_direction _amount) (`Timeline|TL_Dissolve` :!via `PlayFromStart`)
    (:`Update`
      (`MeshComponent.SetScalarParameterValueOnMaterials` (`self.Mesh`) "Dissolve" _amount))
    (:`Finished`
      (`self.K2_DestroyActor`))))

(fn `UserConstructionScript`)