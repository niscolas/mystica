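; Master gameplay ability for enemy hit reactions, activated by a gameplay event.
; It optionally snaps the avatar's rotation to look at the event's instigator, then plays a random montage from its Montages array.
; The ability ends when the montage completes, blends out or is interrupted or cancelled, or after a short delay if the array is empty.
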(event `self.K2_ActivateAbilityFromEvent`
  (params (EventData :type "GameplayEventData Structure (by ref)"))
  (`self.FaceAttackerIfNeeded` EventData)
  (if (not (`KismetArrayLibrary.Array_IsEmpty` (`self.Montages`)))
    (`self.PlayMontage`)
    (else
      (`KismetSystemLibrary.Delay` 0.2)
      (`self.K2_EndAbility`))))

(fn `FaceAttackerIfNeeded`
  (params (GameplayEventData :type "GameplayEventData Structure (by ref)"))
  (bind _returnvalue (`self.GetAvatarActorFromActorInfo`))
  (if (`self.ShouldFaceAttacker`)
    (`Actor.K2_SetActorRotation` _returnvalue (`KismetMathLibrary.FindLookAtRotation` (`Actor.K2_GetActorLocation` _returnvalue) (`Actor.K2_GetActorLocation` (`.Instigator` (break `GameplayEventData` GameplayEventData)))) false)))