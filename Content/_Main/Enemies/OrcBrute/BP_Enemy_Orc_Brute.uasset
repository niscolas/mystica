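; Orc Brute enemy Blueprint that inherits its behavior from a parent class and carries an Ability System Component.
; Tick calls the parent, then prints a gameplay attribute value from that component every frame, apparently as debug output.
; BeginPlay and overlap events are disabled placeholders, and the construction script only calls the parent.
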(event `self.ReceiveTick`
  (params (DeltaSeconds :type "Float (single-precision)"))
  (`parent.ReceiveTick` DeltaSeconds)
  (`KismetSystemLibrary.PrintString` (`KismetStringLibrary.Conv_DoubleToString` (`.ReturnValue` (`AbilitySystemComponent.GetGameplayAttributeValue` (`self.AbilitySystemComponent`) (struct :`AttributeName` "MaxHealth" :`Attribute` "/Script/Mystica.MysticaAttributeSet:MaxHealth" :`AttributeOwner` "/Script/CoreUObject.Class'/Script/Mystica.MysticaAttributeSet'"))))))

(fn `UserConstructionScript`
  (`parent.UserConstructionScript`))