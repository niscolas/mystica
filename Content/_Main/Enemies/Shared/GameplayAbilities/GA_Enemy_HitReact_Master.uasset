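; Master gameplay ability for enemy hit reactions, activated from a gameplay event.
; On activation it optionally turns the avatar toward the event instigator, applies an outline overlay material and plays a random montage if any are set.
; It applies the under-attack status effect to itself, then ends after a short fixed delay independent of montage callbacks, clearing the overlay on end.
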(event `self.K2_ActivateAbilityFromEvent`
  (params (EventData :type "GameplayEventData Structure (by ref)"))
  (`self.FaceAttackerIfNeeded` EventData)
  (`MeshComponent.SetOverlayMaterial` (`self.GetOwningComponentFromActorInfo`) "/Game/_Main/Libraries/MaterialLibrary/M_OutlineOverlay.M_OutlineOverlay")
  (if (not (`KismetArrayLibrary.Array_IsEmpty` (`self.Montages`)))
    (`self.PlayMontage`
      (:` `
        _)))
  (`self.K2_ApplyGameplayEffectSpecToOwner` (`self.MakeOutgoingGameplayEffectSpec` "/Game/_Main/Enemies/Shared/GE_Enemy_AddUnderAttackStatus.GE_Enemy_AddUnderAttackStatus_C"))
  (`KismetSystemLibrary.Delay` 0.2)
  (`self.K2_EndAbility`))

(event `self.K2_OnEndAbility`
  (params (bWasCancelled :type Boolean))
  (`MeshComponent.SetOverlayMaterial` (`self.GetOwningComponentFromActorInfo`) null))

(fn `FaceAttackerIfNeeded`
  (params (GameplayEventData :type "GameplayEventData Structure (by ref)"))
  (bind _returnvalue (`self.GetAvatarActorFromActorInfo`))
  (if (`self.ShouldFaceAttacker`)
    (`Actor.K2_SetActorRotation` _returnvalue (`KismetMathLibrary.FindLookAtRotation` (`Actor.K2_GetActorLocation` _returnvalue) (`Actor.K2_GetActorLocation` (`.Instigator` (break `GameplayEventData` GameplayEventData)))) false)))