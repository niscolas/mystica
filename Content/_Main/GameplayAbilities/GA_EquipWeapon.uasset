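; GA_EquipWeapon is a gameplay ability that equips the player's weapon identified by a weapon tag.
; It plays an interact montage and, on a gameplay event, attaches the weapon component to a socket on the owning component.
; It then links the weapon's anim layer, adds its input mapping context, grants its abilities and registers it as equipped with the combat component.
; The ability ends when the montage completes, blends out or is interrupted or cancelled.
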(event `self.K2_ActivateAbility`
  (bind _returnvalue (`CombatComponent.GetWeaponByTag` (`self.GetCombatComponentFromActorInfo`) (`self.WeaponTag`)))
  (`AbilityTask_PlayMontageAndWait.CreatePlayMontageAndWaitProxy` "None" "/Game/_Main/Player/Animation/AM_InteractLeft.AM_InteractLeft"
    (:`then`
      (`AbilityTask_WaitGameplayEvent.WaitGameplayEvent` (`self.EventTag`) null
        (:`EventReceived`
          (`/Engine/EditorBlueprintResources/StandardMacros.IsValid` _returnvalue
            (:`Is Valid`
              (`Actor.K2_AttachToComponent` _returnvalue (`self.GetOwningComponentFromActorInfo`) (`self.WeaponSocket`) "SnapToTarget" "KeepRelative" "KeepWorld" true)
              (`self.Handle Weapon Equipping`))))))
    (:`OnCompleted`
      (`self.K2_EndAbility` :!label _label))
    (:`OnBlendOut`
      (goto _label))
    (:`OnInterrupted`
      (goto _label))
    (:`OnCancelled`
      (goto _label))))

(fn `Handle Weapon Equipping`
  (locals (Weapon :type "PlayerWeaponComponent Object Reference"))
  (set `local.Weapon` (`PlayerCombatComponent.GetPlayerWeaponComponentByTag` (cast `PlayerCombatComponent` (`self.GetCombatComponentFromActorInfo`) :!pure true) (`self.WeaponTag`)))
  (`|ExecutionSequence`
    (:`then_0`
      (`SkeletalMeshComponent.LinkAnimClassLayers` (`self.GetOwningComponentFromActorInfo`) (`PlayerWeaponComponent.LinkedAnimLayer` (`local.Weapon`))))
    (:`then_1`
      (`EnhancedInputSubsystemInterface.AddMappingContext` (pcsubsystem `EnhancedInputLocalPlayerSubsystem` (`self.GetPlayerControllerFromActorInfo`)) (`PlayerWeaponComponent.EquippedInputMappingContext` (`local.Weapon`)) 1 (struct)))
    (:`then_2`
      (`MysticaAbilitySystemComponent.GrantWeaponAbilities` (`self.GetPlayerAbilitySystemComponentFromActorInfo`) (`PlayerWeaponComponent.DefaultAbilities` (`local.Weapon`)) (`self.GetAbilityLevel`)))
    (:`then_3`
      (`CombatComponent.EquipWeapon` (`self.GetCombatComponentFromActorInfo`) (`self.WeaponTag`)))))